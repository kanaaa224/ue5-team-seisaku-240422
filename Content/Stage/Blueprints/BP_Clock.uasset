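; BP_Clock is a stage countdown timer that starts when play begins.
; DecSec waits one second, decrements TimeLimiteSeconds and prints the remaining time, then calls itself again until the count reaches zero.
; At zero or below it stops looping and calls CallTimeLimite to signal that time is up.
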(event `self.ReceiveBeginPlay`
  (`self.DecSec`))

(event `DecSec`
  (`KismetSystemLibrary.Delay` 1.0)
  (bind _result (`/Engine/EditorBlueprintResources/StandardMacros.DecrementInt` (`self.TimeLimiteSeconds`))
    (:`  `
      (`KismetSystemLibrary.PrintString` (`KismetStringLibrary.Concat_StrStr` "TimeLimite" (`KismetStringLibrary.Conv_IntToString` _result)))
      (if (<= (`self.TimeLimiteSeconds`) 0)
        (`self.TimeLimite`)
        (else
          (`self.DecSec`))))))

(fn `UserConstructionScript`)