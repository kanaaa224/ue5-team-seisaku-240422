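; BP_Booom is a stage actor that explodes the first time it takes any damage.
; It hides its particle system on BeginPlay.
; On damage, it fires a RadialForce impulse, then reveals and activates the particle effect.
; An IsBoom flag limits the explosion to a single trigger, and the actor is not destroyed afterward.
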(event `self.ReceiveBeginPlay`
  (`SceneComponent.SetVisibility` (`self.ParticleSystem`) false false))

(event `self.ReceiveAnyDamage`
  (params (Damage :type "Float (single-precision)") (DamageType :type "DamageType Object Reference") (InstigatedBy :type "Controller Object Reference") (DamageCauser :type "Actor Object Reference"))
  (if (not (`self.Is Boom`))
    (set `self.Is Boom` true)
    (`RadialForceComponent.FireImpulse` (`self.RadialForce`))
    (`SceneComponent.SetVisibility` (`self.ParticleSystem`) true false)
    (`ActorComponent.Activate` (`self.ParticleSystem`) false)))

(fn `UserConstructionScript`)