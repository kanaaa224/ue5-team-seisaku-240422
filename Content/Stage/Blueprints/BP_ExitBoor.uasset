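; Exit door actor that runs an exit countdown while a team 1 player stands in its trigger box.
; A recursive one-second delay loop decrements and prints Seconds, then calls CallExit once it drops below zero.
; Countdown thresholds light three pairs of point lights alongside a red light, turning the pairs blue at zero.
; Any player leaving the box pauses the countdown without resetting it, darkens the lights and stops the warning sound.
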(event `self.ReceiveBeginPlay`
  (`self.Light Off`)
  (`AudioComponent.Stop` (`self.Warning Sound`)))

(event `Light Off`
  (set `self.Is Light On` false)
  (`SceneComponent.SetVisibility` (`self.PointLight3`) false false)
  (`SceneComponent.SetVisibility` (`self.PointLight2`) false false)
  (`SceneComponent.SetVisibility` (`self.PointLight1`) false false)
  (`SceneComponent.SetVisibility` (`self.PointLight6`) false false)
  (`SceneComponent.SetVisibility` (`self.PointLight5`) false false)
  (`SceneComponent.SetVisibility` (`self.PointLight4`) false false)
  (`SceneComponent.SetVisibility` (`self.PL_Red`) false false))

(event `Light On`
  (set `self.Is Light On` true)
  (`SceneComponent.SetVisibility` (`self.PL_Red`) true false)
  (if (`self.First Light On`)
    (`SceneComponent.SetVisibility` (`self.PointLight1`) true false)
    (`SceneComponent.SetVisibility` (`self.PointLight6`) true false))
  (if (`self.Second Light On`)
    (`SceneComponent.SetVisibility` (`self.PointLight2`) true false)
    (`SceneComponent.SetVisibility` (`self.PointLight5`) true false))
  (if (`self.Third Light On`)
    (`SceneComponent.SetVisibility` (`self.PointLight3`) true false)
    (`SceneComponent.SetVisibility` (`self.PointLight4`) true false)
    (`LightComponent.SetLightColor` (`self.PointLight1`) (struct :`B` 1.0 :`A` 1.0) true)
    (`LightComponent.SetLightColor` (`self.PointLight2`) (struct :`B` 1.0 :`A` 1.0) true)
    (`LightComponent.SetLightColor` (`self.PointLight3`) (struct :`B` 1.0 :`A` 1.0) true)
    (`LightComponent.SetLightColor` (`self.PointLight4`) (struct :`B` 1.0 :`A` 1.0) true)
    (`LightComponent.SetLightColor` (`self.PointLight5`) (struct :`B` 1.0 :`A` 1.0) true)
    (`LightComponent.SetLightColor` (`self.PointLight6`) (struct :`B` 1.0 :`A` 1.0) true)))

(event `Dec Seconds`
  (if (`self.Is Overlap`)
    (if (< (`self.Seconds`) 0)
      (set `self.Is Exit` true)
      (`self.Exit`)
      (else
        (`KismetSystemLibrary.Delay` 1.0)
        (bind _output_get (set `self.Seconds` (- (`self.Seconds`) 1)))
        (`KismetSystemLibrary.PrintString` (`KismetStringLibrary.Concat_StrStr` "Exit Seconds : " (`KismetStringLibrary.Conv_IntToString` _output_get)) true true (struct :`G` 1.0 :`B` 0.102637 :`A` 1.0) 1.0)
        (if (<= (`self.Seconds`) 40)
          (set `self.First Light On` true))
        (if (<= (`self.Seconds`) 20)
          (set `self.Second Light On` true))
        (if (<= (`self.Seconds`) 0)
          (set `self.Third Light On` true))
        (`self.Dec Seconds`)
        (`self.Light On`)))))

(event `self.Box.OnComponentBeginOverlap`
  (params (OverlappedComponent :type "PrimitiveComponent Object Reference") (OtherActor :type "Actor Object Reference") (OtherComp :type "PrimitiveComponent Object Reference") (OtherBodyIndex :type Integer) (bFromSweep :type Boolean) (SweepResult :type "HitResult Structure (by ref)"))
  (bind _asbp_first_person (cast `/Game/Player/FirstPerson/Blueprints/BP_FirstPerson` OtherActor))
  (if (== (`/Game/System/Blueprints/PlayerState_1.TeamID` (cast `/Game/System/Blueprints/PlayerState_1` (`Pawn.PlayerState` _asbp_first_person) :!pure true)) 1)
    (set `self.Is Overlap` true)
    (`self.Dec Seconds`)
    (`AudioComponent.Play` (`self.Warning Sound`) 0.0)))

(event `self.Box.OnComponentEndOverlap`
  (params (OverlappedComponent :type "PrimitiveComponent Object Reference") (OtherActor :type "Actor Object Reference") (OtherComp :type "PrimitiveComponent Object Reference") (OtherBodyIndex :type Integer))
  (cast `/Game/Player/FirstPerson/Blueprints/BP_FirstPerson` OtherActor)
  (set `self.Is Overlap` false)
  (`self.Light Off`)
  (`AudioComponent.Stop` (`self.Warning Sound`)))

(fn `UserConstructionScript`)