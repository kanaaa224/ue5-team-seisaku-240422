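; Main multiplayer game mode that manages player admission, two-team spawning, respawns and the trip to the matching room.
; Post-login kicks players beyond the GameInstance's MaxPlayers and loads saved game state once full; later logouts reset that limit.
; Spawns pick a random PlayerStart tagged with the player's TeamID, while a separate counter alternates team IDs.
; OpenLevel saves state through the GameInstance, then server-travels to Level_MatchingRoom.
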(event `self.ReceiveBeginPlay`)

(event `PlayerDied` :!signature `self.OnPlayerDied`
  (params (Character :type "Character Object Reference"))
  (`self.RestartPlayer` (`Pawn.GetController` Character)))

(event `UpdateTeamID`
  (bind _latestallocatedteamid (`self.LatestAllocatedTeamID`))
  (`/Engine/EditorBlueprintResources/StandardMacros.IncrementInt` _latestallocatedteamid
    (:`  `
      (set `self.LatestAllocatedTeamID` (mod _latestallocatedteamid 2)))))

(event `self.K2_PostLogin`
  (params (NewPlayer :type "PlayerController Object Reference"))
  (`|ExecutionSequence`
    (:`then_0`
      (bind _asgame_instance_main (cast `/Game/System/Blueprints/GameInstance_Main` (`GameplayStatics.GetGameInstance`)))
      (bind _players (`self.GetCurrentPlayers`))
      (if (> _players (`/Game/System/Blueprints/GameInstance_Main.MaxPlayers` _asgame_instance_main))
        (bind _asplayer_controller_main (cast `/Game/System/Blueprints/PlayerController_Main` (`GameplayStatics.GetPlayerController` (- _players 1))))
        (`/Game/System/Blueprints/PlayerController_Main.Kick` _asplayer_controller_main)))
    (:`then_1`
      (bind _asgame_instance_main_2 (cast `/Game/System/Blueprints/GameInstance_Main` (`GameplayStatics.GetGameInstance`)))
      (bind _players_2 (`self.GetCurrentPlayers`))
      (if (== _players_2 (`/Game/System/Blueprints/GameInstance_Main.MaxPlayers` _asgame_instance_main_2))
        (`/Game/System/Blueprints/GameInstance_Main.LoadGameState` _asgame_instance_main_2)
        (set `self.isAllPlayerLoggedIn` true)))))

(event `self.K2_OnLogout`
  (params (ExitingController :type "Controller Object Reference"))
  (if (`self.isAllPlayerLoggedIn`)
    (bind _asgame_instance_main (cast `/Game/System/Blueprints/GameInstance_Main` (`GameplayStatics.GetGameInstance`)))
    (bind _players (`self.GetCurrentPlayers`))
    (set `/Game/System/Blueprints/GameInstance_Main.MaxPlayers` _players _asgame_instance_main)))

(event `OpenLevel`
  (bind _asgame_instance_main (cast `/Game/System/Blueprints/GameInstance_Main` (`GameplayStatics.GetGameInstance`)))
  (`/Game/System/Blueprints/GameInstance_Main.SaveGameState` _asgame_instance_main)
  (`KismetSystemLibrary.ExecuteConsoleCommand` (`KismetStringLibrary.Concat_StrStr` "servertravel " "/Game/UI/Maps/Level_MatchingRoom") (`GameplayStatics.GetPlayerController` 0)))

(fn `ChoosePlayerStart`
  (params (Player :type "Controller Object Reference"))
  (returns (ReturnValue :type "Actor Object Reference"))
  (bind _asplayer_state_main (cast `/Game/System/Blueprints/PlayerState_Main` (`Controller.PlayerState` Player)))
  (bind (_statedata_ishost _statedata_isready _statedata_playername _statedata_teamid) (break `/Game/System/Blueprints/Struct_PlayerStateData` (`/Game/System/Blueprints/PlayerState_Main.StateData` _asplayer_state_main)))
  (bind _outactors (`GameplayStatics.GetAllActorsOfClassWithTag` "/Script/Engine.PlayerStart" (`KismetStringLibrary.Conv_StringToName` (`KismetStringLibrary.Conv_IntToString` _statedata_teamid))))
  (return (`KismetArrayLibrary.Array_Random` _outactors)))

(fn `GetCurrentPlayers`
  (returns (Players :type Integer))
  (bind _asgame_state_main (cast `/Game/System/Blueprints/GameState_Main` (`GameplayStatics.GetGameState`)))
  (for (_ _array_index) (`GameStateBase.PlayerArray` _asgame_state_main)
    _)
  (return (+ _array_index 1)))

(fn `UserConstructionScript`)