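; BP_Light_1 is a stage light that goes dark for a while when it takes any damage.
; The damage event calls a custom OnServer event, which activates the particle system and hides the spot and point lights.
; After a fixed delay of a few seconds, both lights become visible again.
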(event `self.ReceiveAnyDamage`
  (params (Damage :type "Float (single-precision)") (DamageType :type "DamageType Object Reference") (InstigatedBy :type "Controller Object Reference") (DamageCauser :type "Actor Object Reference"))
  (`self.On Server`))

(event `On Server`
  (`ActorComponent.Activate` (`self.ParticleSystem`) false)
  (`SceneComponent.SetVisibility` (`self.SpotLight`) false false)
  (`SceneComponent.SetVisibility` (`self.PointLight`) false false)
  (`KismetSystemLibrary.Delay` 7.0)
  (`SceneComponent.SetVisibility` (`self.SpotLight`) true false)
  (`SceneComponent.SetVisibility` (`self.PointLight`) true false))

(fn `UserConstructionScript`)