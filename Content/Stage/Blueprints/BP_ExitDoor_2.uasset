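; BP_ExitDoor_2 is an exit door that counts down while the first-person player stands in its Box trigger.
; Overlap starts a warning sound and three lights, and leaving stops both.
; DecSeconds re-calls itself through a one-second Delay, lowering Seconds while overlap lasts, then sets CanExit once it drops below zero.
; Leaving pauses the countdown without resetting it, and progress shows only as debug prints.
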(event `Light Off`
  (set `self.Is Light On` false)
  (`SceneComponent.SetVisibility` (`self.PointLight`) false false)
  (`SceneComponent.SetVisibility` (`self.SpotLight`) false false)
  (`SceneComponent.SetVisibility` (`self.SpotLight1`) false false))

(event `Ligth On`
  (set `self.Is Light On` true)
  (`SceneComponent.SetVisibility` (`self.PointLight`) true false)
  (`SceneComponent.SetVisibility` (`self.SpotLight`) true false)
  (`SceneComponent.SetVisibility` (`self.SpotLight1`) true false))

(event `Dec Seconds`
  (if (`self.is OverlapDoor`)
    (if (< (`self.Seconds`) 0.0)
      (set `self.Can Exit` true)
      (`KismetSystemLibrary.PrintString` "Exit!!")
      (elif (not (`self.Can Exit`))
        (`KismetSystemLibrary.Delay` 1.0)
        (bind _output_get (set `self.Seconds` (- (`self.Seconds`) (`self.Dec Value`))))
        (`KismetSystemLibrary.PrintString` (`KismetStringLibrary.Concat_StrStr` "Exit Seconds : " (`KismetStringLibrary.Conv_DoubleToString` _output_get)) true true (struct :`G` 1.0 :`B` 0.102637 :`A` 1.0) 1.0)
        (`self.Dec Seconds`)))))

(event `self.Box.OnComponentBeginOverlap`
  (params (OverlappedComponent :type "PrimitiveComponent Object Reference") (OtherActor :type "Actor Object Reference") (OtherComp :type "PrimitiveComponent Object Reference") (OtherBodyIndex :type Integer) (bFromSweep :type Boolean) (SweepResult :type "HitResult Structure (by ref)"))
  (cast `/Game/Player/FirstPerson/Blueprints/BP_FirstPerson` OtherActor)
  (set `self.is OverlapDoor` true)
  (`self.Dec Seconds`)
  (`KismetSystemLibrary.PrintString` "Begin Dec Seconds")
  (`AudioComponent.Play` (`self.Warning_Audio`) 0.0)
  (`self.Ligth On`))

(event `self.Box.OnComponentEndOverlap`
  (params (OverlappedComponent :type "PrimitiveComponent Object Reference") (OtherActor :type "Actor Object Reference") (OtherComp :type "PrimitiveComponent Object Reference") (OtherBodyIndex :type Integer))
  (cast `/Game/Player/FirstPerson/Blueprints/BP_FirstPerson` OtherActor)
  (set `self.is OverlapDoor` false)
  (`KismetSystemLibrary.PrintString` "Stop Dec Seconds")
  (`self.Light Off`)
  (`AudioComponent.Stop` (`self.Warning_Audio`)))

(event `self.ReceiveBeginPlay`
  (`self.Light Off`)
  (`AudioComponent.Stop` (`self.Warning_Audio`)))

(fn `UserConstructionScript`)