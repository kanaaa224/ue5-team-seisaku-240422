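; PlayerState_1 is a player state Blueprint that holds a player's ready flag, name and team ID.
; Three setter events write those values directly.
; Its construction script casts the game mode to GameMode_1, takes its latest allocated team ID, then calls UpdateTeamID on it.
; Team assignment therefore happens at construction, and only where that cast succeeds.
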(event `SetReadyState`
  (params (readyState :type Boolean))
  (set `self.IsReady` readyState))

(event `SetPlayerName`
  (params (playerName :type String))
  (set `self.PlayerName` playerName))

(event `SetTeamID`
  (params (teamID :type Integer))
  (set `self.TeamID` teamID))

(fn `UserConstructionScript`
  (bind _asgame_mode_1 (cast `/Game/System/Blueprints/GameMode_1` (`GameplayStatics.GetGameMode`)))
  (set `self.TeamID` (`/Game/System/Blueprints/GameMode_1.LatestAllocatedTeamID` _asgame_mode_1))
  (`/Game/System/Blueprints/GameMode_1.UpdateTeamID` _asgame_mode_1))