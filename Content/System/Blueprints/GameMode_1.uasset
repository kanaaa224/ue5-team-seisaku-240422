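; Game mode for a two-team multiplayer game, handling player spawns, team ID allocation and a player-count limit.
; ChoosePlayerStart picks a random PlayerStart tagged with the player's TeamID, and UpdateTeamID alternates the latest allocated ID between two teams.
; PostLogin kicks the controller at the last player index when the GameState player count exceeds the GameInstance's CurrentPlayers.
; PlayerDied restarts the player, but its dispatcher binding is unconnected.
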(event `self.ReceiveBeginPlay`)

(event `PlayerDied` :!signature `self.OnPlayerDied`
  (params (Character :type "Character Object Reference"))
  (`self.RestartPlayer` (`Pawn.GetController` Character)))

(event `UpdateTeamID`
  (bind _latestallocatedteamid (`self.latestAllocatedTeamID`))
  (`/Engine/EditorBlueprintResources/StandardMacros.IncrementInt` _latestallocatedteamid
    (:`  `
      (set `self.latestAllocatedTeamID` (mod _latestallocatedteamid 2)))))

(event `self.K2_PostLogin`
  (params (NewPlayer :type "PlayerController Object Reference"))
  (bind _asgame_instance_1 (cast `/Game/System/Blueprints/GameInstance_1` (`GameplayStatics.GetGameInstance`)))
  (bind _players (`self.GetCurrentPlayers`))
  (if (> _players (`/Game/System/Blueprints/GameInstance_1.currentPlayers` _asgame_instance_1))
    (bind _asplayer_controller_1 (cast `/Game/System/Blueprints/PlayerController_1` (`GameplayStatics.GetPlayerController` (- _players 1))))
    (`/Game/System/Blueprints/PlayerController_1.Kick` _asplayer_controller_1)))

(fn `ChoosePlayerStart`
  (params (Player :type "Controller Object Reference"))
  (returns (ReturnValue :type "Actor Object Reference"))
  (bind _asplayer_state_1 (cast `/Game/System/Blueprints/PlayerState_1` (`Controller.PlayerState` Player)))
  (bind _outactors (`GameplayStatics.GetAllActorsOfClassWithTag` "/Script/Engine.PlayerStart" (`KismetStringLibrary.Conv_StringToName` (`KismetStringLibrary.Conv_IntToString` (`/Game/System/Blueprints/PlayerState_1.TeamID` _asplayer_state_1)))))
  (return (`KismetArrayLibrary.Array_Random` _outactors)))

(fn `GetCurrentPlayers`
  (returns (Players :type Integer))
  (bind _asgame_state_1 (cast `/Game/System/Blueprints/GameState_1` (`GameplayStatics.GetGameState`)))
  (for (_ _array_index) (`GameStateBase.PlayerArray` _asgame_state_1)
    _)
  (return (+ _array_index 1)))

(fn `UserConstructionScript`)